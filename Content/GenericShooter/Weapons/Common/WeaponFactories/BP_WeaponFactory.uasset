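; BP_WeaponFactory is a networked weapon spawner that offers a WeaponClass pickup at WeaponSpawnPoint and respawns it after it is taken.
; The server spawns the weapon with mesh physics off, either shortly after BeginPlay or after RespawnTimer, and restarts that timer on pickup.
; SpawnedWeapon's RepNotify lets clients snap and attach the weapon to the spawn point and toggle the particle effect.
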(event EventBeginPlay
  (Networking|SwitchHasAuthority
    (:Authority
      (Utilities|FlowControl|Delay 1.0)
      (if (Variables|Default|GetbSpawnOnStart)
        (CallFunction|SpawnWeapon)
        (else
          (CallFunction|StartRespawn))))
    (:Remote
      (CallFunction|ResetSpawnedWeaponVisuals))))

(fn ConstructionScript)

(fn SpawnWeapon
  (Networking|SwitchHasAuthority
    (:Authority
      (if (not (Utilities|IsValid (Variables|Default|GetSpawnedWeapon)))
        (bind _returnvalue (Game|SpawnActorfromClass (Variables|Default|GetWeaponClass) (Transformation|GetWorldTransform (Variables|Default|GetWeaponSpawnPoint)) "AlwaysSpawn" self false 0))
        (Variables|Default|SetSpawnedWeapon _returnvalue)
        (Physics|SetSimulatePhysics (Variables|/Game/GenericShooter/BlueprintLogic/Weapons/BP_BaseWeapon.BP_BaseWeapon_C|Get3PMesh _returnvalue) false)
        (Collision|SetCollisionResponsetoChannel (Variables|/Game/GenericShooter/BlueprintLogic/Weapons/BP_BaseWeapon.BP_BaseWeapon_C|Get3PMesh _returnvalue) "ECC_GameTraceChannel1" "ECR_Ignore")
        (EventDispatchers|BindEventtoOnWeaponPickedUp _returnvalue (EventDispatchers|CreateEvent self :!event OnWeaponPickedUp))
        (Components|Activation|SetActive (Variables|Default|GetParticleSystem) true true)
        (Variables|/Script/Engine.SceneComponent|SetbUseAttachParentBound (Variables|/Game/GenericShooter/BlueprintLogic/Weapons/BP_BaseWeapon.BP_BaseWeapon_C|Get3PMesh _returnvalue) false)))))

(fn OnWeaponPickedUp
  (EventDispatchers|UnbindallEventsfromOnWeaponPickedUp (Variables|Default|GetSpawnedWeapon))
  (Variables|Default|SetSpawnedWeapon 0)
  (CallFunction|StartRespawn)
  (Components|Activation|SetActive (Variables|Default|GetParticleSystem) false false))

(fn StartRespawn
  (Networking|SwitchHasAuthority
    (:Authority
      (Utilities|Time|SetTimerbyFunctionName 0 "SpawnWeapon" (Variables|Default|GetRespawnTimer)))))

(fn OnRepSpawnedWeapon
  (CallFunction|ResetSpawnedWeaponVisuals))

(fn ResetSpawnedWeaponVisuals
  (bind _particlesystem (Variables|Default|GetParticleSystem))
  (bind _spawnedweapon (Variables|Default|GetSpawnedWeapon))
  (bind _weaponspawnpoint (Variables|Default|GetWeaponSpawnPoint))
  (bind _3pmesh (Variables|/Game/GenericShooter/BlueprintLogic/Weapons/BP_BaseWeapon.BP_BaseWeapon_C|Get3PMesh _spawnedweapon))
  (Utilities|IsValid _spawnedweapon
    (:Is%20Valid
      (Physics|SetSimulatePhysics _3pmesh false)
      (Transformation|SetActorLocation _spawnedweapon (Transformation|GetWorldLocation _weaponspawnpoint) false false)
      (Transformation|SetActorRotation _spawnedweapon (Transformation|GetWorldRotation _weaponspawnpoint))
      (Class|Actor|AttachRootComponentto _spawnedweapon (Variables|Default|GetWeaponSpawnPoint) "None" "KeepWorldPosition" true)
      (Variables|/Script/Engine.SceneComponent|SetbUseAttachParentBound (Variables|/Game/GenericShooter/BlueprintLogic/Weapons/BP_BaseWeapon.BP_BaseWeapon_C|Get3PMesh _spawnedweapon) false)
      (Collision|SetCollisionResponsetoChannel _3pmesh "ECC_GameTraceChannel1" "ECR_Ignore")
      (Components|Activation|Activate _particlesystem true))
    (:Is%20Not%20Valid
      (Components|Activation|Deactivate _particlesystem)))
  (return))